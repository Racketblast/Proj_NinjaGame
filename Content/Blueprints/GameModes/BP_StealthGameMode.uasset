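; BP_StealthGameMode is a game mode that shows the end-game screen once the fifth mission has been cleared.
; On BeginPlay it reads the cleared missions and finished flag from the StealthGameInstance.
; If the game is not yet marked finished, it sets that flag so the screen shows only once, then adds the end-game widget to the viewport after a zero-length delay.
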(event EventBeginPlay
  (bind _asstealth_game_instance (Utilities|Casting|CastToStealthGameInstance (Game|GetGameInstance)))
  (if (and (not (Variables|/Script/Proj_NinjaGame.StealthGameInstance|GetbFinishedTheGame _asstealth_game_instance)) (Utilities|Array|ContainsItem (Variables|/Script/Proj_NinjaGame.StealthGameInstance|GetMissionsCleared _asstealth_game_instance) "FifthMission"))
    (Variables|/Script/Proj_NinjaGame.StealthGameInstance|SetbFinishedTheGame _asstealth_game_instance true)
    (Utilities|FlowControl|Delay 0.0)
    (bind _returnvalue (UserInterface|CreateWidget (Variables|Default|GetEndGameWidgetClass)))
    (UserInterface|Viewport|AddtoViewport _returnvalue 0)))

(event EventTick
  (params (DeltaSeconds :type Float%20%28single-precision%29)))

(fn ConstructionScript)
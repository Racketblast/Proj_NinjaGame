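; BP_StealthPlayerController is a player controller for the stealth game that handles pause input and a progression-unlock hotkey.
; The IA_PauseMenu input action creates a new PauseMenu widget and adds it to the viewport.
; Pressing L acts as an apparent debug cheat, adding every missing EMission value to the StealthGameInstance's MissionsCleared, then setting CurrentGameFlag to a very high value.
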(event Input|EnhancedActionEvents|EnhancedInputActionIA_PauseMenu
  (params (ActionValue :type Boolean) (ElapsedSeconds :type Float%20%28double-precision%29) (TriggeredSeconds :type Float%20%28double-precision%29) (InputAction :type Input%20Action%20Object%20Reference :default "/Game/Input/Actions/IA_PauseMenu.IA_PauseMenu"))
  (bind _returnvalue (UserInterface|CreateWidget "/Game/UI_Elements/UI_Widgets/Menus/PauseMenu.PauseMenu_C"))
  (UserInterface|Viewport|AddtoViewport _returnvalue 0))

(event EventBeginPlay)

(event EventTick
  (params (DeltaSeconds :type Float%20%28single-precision%29)))

(event Input|KeyboardEvents|L
  (params (Key :type Key%20Structure :default "None"))
  (:Pressed
    (bind _asstealth_game_instance (Utilities|Casting|CastToStealthGameInstance (Game|GetGameInstance)))
    (bind _enumvalue (|ForEachEMission)
      (:LoopBody
        (if (not (Utilities|Array|ContainsItem (Variables|/Script/Proj_NinjaGame.StealthGameInstance|GetMissionsCleared _asstealth_game_instance) _enumvalue))
          (Utilities|Array|Add (Variables|/Script/Proj_NinjaGame.StealthGameInstance|GetMissionsCleared _asstealth_game_instance) _enumvalue)))
      (:then
        (Variables|/Script/Proj_NinjaGame.StealthGameInstance|SetCurrentGameFlag _asstealth_game_instance 9999)))))

(fn ConstructionScript)
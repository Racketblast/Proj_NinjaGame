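; BP_FootstepsNotify is an animation notify that plays footstep sounds for the StealthCharacter, with volume set by movement state.
; Walk, run and crouch each supply a leg length and a volume multiplier.
; A visibility line trace that long below the actor checks for ground and returns that multiplier as the volume of PlaySoundAtLocation.
; The surface type is queried, but the sound is always the carpet step.
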(fn ReceivedNotify
  (params (MeshComp :type Skeletal%20Mesh%20Component%20Object%20Reference) (Animation :type Anim%20Sequence%20Base%20Object%20Reference) (EventReference :type Anim%20Notify%20Event%20Reference%20Structure%20%28by%20ref%29))
  (bind _asstealth_character (Utilities|Casting|CastToStealthCharacter (Components|GetOwner MeshComp)))
  (bind _volumemodifier (CallFunction|TraceTouchesGround _asstealth_character))
  (Audio|PlaySoundatLocation "/Game/Audio/PlayerSounds/Footsteps/SC_CarpetStep.SC_CarpetStep" "0, 0, 0" "0, 0, 0" _volumemodifier 1.0 0.0 0 0 0 0)
  (return false))

(fn TraceTouchesGround
  (params (Player :type Stealth%20Character%20Object%20Reference))
  (bind _returnvalue (Transformation|GetActorLocation Player))
  (bind (_leglength _soundmultiplier) (CallFunction|GetStanceFloats (Variables|/Script/Proj_NinjaGame.StealthCharacter|GetCurrentMovementState Player)))
  (bind (_outhit _returnvalue_2) (Collision|LineTraceByChannel _returnvalue (+ _returnvalue (* (Transformation|GetActorUpVector Player) _leglength)) "TraceTypeQuery1" false 0 "None"))
  (if _returnvalue_2
    (switch Utilities|FlowControl|Switch|SwitchonEPhysicalSurface (Collision|GetSurfaceType _outhit)
      (:SurfaceType_Default
        (return _soundmultiplier)))))

(fn GetStanceFloats
  (params (State :type EPlayerMovementState%20Enum :default "Walk"))
  (switch Utilities|FlowControl|Switch|SwitchonEPlayerMovementState State
    (:Walk
      (return -125.0 0.5))
    (:Run
      (return -125.0 0.8))
    (:Crouch
      (return -75.0 0.3))))
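; BP_AIFootsteps is an animation notify that plays footstep audio for MeleeEnemy characters.
; On notify, it line traces 150 units down from the owning actor on the Visibility channel and switches on the hit surface type.
; The only sound shown is SC_CarpetStep, which it sets and plays on the enemy's FootstepsAudioComponent after casting the owner.
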(fn ReceivedNotify
  (params (MeshComp :type Skeletal%20Mesh%20Component%20Object%20Reference) (Animation :type Anim%20Sequence%20Base%20Object%20Reference) (EventReference :type Anim%20Notify%20Event%20Reference%20Structure%20%28by%20ref%29))
  (bind _returnvalue (Components|GetOwner MeshComp))
  (bind _returnvalue_2 (Transformation|GetActorLocation _returnvalue))
  (bind (_outhit _returnvalue_3) (Collision|LineTraceByChannel _returnvalue_2 (+ _returnvalue_2 (* (Transformation|GetActorUpVector _returnvalue) -1.5e+02)) "TraceTypeQuery1" false 0 "None"))
  (if _returnvalue_3
    (switch Utilities|FlowControl|Switch|SwitchonEPhysicalSurface (Collision|GetSurfaceType _outhit)
      (:SurfaceType_Default
        (bind _asmelee_enemy (Utilities|Casting|CastToMeleeEnemy _returnvalue))
        (Audio|Components|Audio|SetSound (Variables|/Script/Proj_NinjaGame.MeleeEnemy|GetFootstepsAudioComponent _asmelee_enemy) "/Game/Audio/PlayerSounds/Footsteps/SC_CarpetStep.SC_CarpetStep")
        (Audio|Components|Audio|Play (Variables|/Script/Proj_NinjaGame.MeleeEnemy|GetFootstepsAudioComponent _asmelee_enemy) 0.0)
        (return false)))))
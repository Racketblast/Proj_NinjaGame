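; BP_StealthAmbientSound is a music controller that switches between looping stealth music and combat music based on enemy detection.
; BeginPlay finds BP_EnemyHandler and starts the stealth theme on one audio component.
; Tick polls the handler's GetEnemySeesPlayer, using a boolean latch to switch only on changes.
; Detection restarts combat music on a second component and pauses stealth music, which resumes where it paused once detection ends.
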(event EventBeginPlay
  (bind _audiocomponent (Variables|Components|GetAudioComponent))
  (bind _returnvalue (Actor|GetActorOfClass "/Game/Blueprints/AI/BP_EnemyHandler.BP_EnemyHandler_C"))
  (Variables|Default|SetEnemyHandler _returnvalue)
  ;[0.15 0.15 0.15 0.5] Sets the first played Music
  (Audio|Components|Audio|SetSound _audiocomponent "/Game/Audio/Themes/THEME_StealthMusicLOOP.THEME_StealthMusicLOOP")
  (Audio|Components|Audio|Play _audiocomponent 0.0))

(event EventTick
  (params (DeltaSeconds :type Float%20%28single-precision%29))
  (bind _enemyhandler (Variables|Default|GetEnemyHandler))
  (bind _audiocomponent1 (Variables|Default|GetAudioComponent1))
  (Utilities|IsValid _enemyhandler
    (:Is%20Valid
      (if (Class|EnemyHandler|GetEnemySeesPlayer _enemyhandler)
        (if (not (Variables|Default|GetbBattleMusicPlayed))
          ;[0.15 0.15 0.15 0.5] Sets Combat music when seen
          (Variables|Default|SetbBattleMusicPlayed true)
          (Audio|Components|Audio|SetSound _audiocomponent1 "/Game/Audio/Themes/combatMusicTEST.combatMusicTEST")
          (Audio|Components|Audio|Play _audiocomponent1 0.0)
          (Class|AudioComponent|SetPaused _audiocomponent1 false)
          (Class|AudioComponent|SetPaused (Variables|Components|GetAudioComponent) true))
        (elif (Variables|Default|GetbBattleMusicPlayed)
          ;[0.15 0.15 0.15 0.5] Sets Normal music after combat
          (Variables|Default|SetbBattleMusicPlayed false)
          (Class|AudioComponent|SetPaused (Variables|Components|GetAudioComponent) false)
          (Class|AudioComponent|SetPaused (Variables|Default|GetAudioComponent1) true))))))

(fn ConstructionScript)
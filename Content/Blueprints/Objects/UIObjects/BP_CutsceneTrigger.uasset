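; BP_CutsceneTrigger is a placed actor that shows a cutscene widget when the player's StealthCharacter overlaps it.
; On BeginPlay it pre-creates the Cutscene_Widget and passes it the media source, sound and fade type.
; Tick polls for overlap while the game instance's current flag is at or below CutsceneGameFlag.
; It plays any white or black fade-in Level Sequence, waits its duration, adds the widget to the viewport, then destroys itself.
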(event EventBeginPlay
  (bind _asstealth_game_instance (Utilities|Casting|CastToStealthGameInstance (Game|GetGameInstance)))
  (Variables|Default|SetAs%20Stealth%20Game%20Instance _asstealth_game_instance)
  (bind _asstealth_character (Utilities|Casting|CastToStealthCharacter (Game|Player|GetPlayerPawn 0)))
  (Variables|Default|SetAs%20Stealth%20Character _asstealth_character)
  (bind _returnvalue (UserInterface|CreateWidget "/Game/UI_Elements/UI_Widgets/Menus/Cutscene_Widget.Cutscene_Widget_C"))
  (bind _output_get (Variables|Default|SetWidget _returnvalue))
  (Variables|/Game/UI_Elements/UI_Widgets/Menus/Cutscene_Widget.Cutscene_Widget_C|SetMedia%20Source _output_get (Variables|Default|GetMedia%20Source))
  (Variables|/Game/UI_Elements/UI_Widgets/Menus/Cutscene_Widget.Cutscene_Widget_C|SetMedia%20Sound _output_get (Variables|Default|GetMedia%20Sound))
  (Variables|/Game/UI_Elements/UI_Widgets/Menus/Cutscene_Widget.Cutscene_Widget_C|SetFadeType _returnvalue (Variables|Default|GetFadeType)))

(event Collision|EventActorBeginOverlap
  (params (OtherActor :type Actor%20Object%20Reference)))

(event EventTick
  (params (DeltaSeconds :type Float%20%28single-precision%29))
  (bind _fadetype (Variables|Default|GetFadeType))
  (bind _fadesequence (CallFunction|GetFadein _fadetype))
  (if (<= (Variables|/Script/Proj_NinjaGame.StealthGameInstance|GetCurrentGameFlag (Variables|Default|GetAs%20Stealth%20Game%20Instance)) (Variables|Default|GetCutsceneGameFlag))
    (if (Collision|IsOverlappingActor (Variables|Default|GetAs%20Stealth%20Character) :!class /Script/Engine.Actor)
      (if (not (Variables|Default|GetbShowingWidget))
        (Variables|Default|SetbShowingWidget true)
        (Utilities|IsValid _fadesequence
          (:Is%20Valid
            (bind (_outactor _returnvalue) (Sequencer|Player|CreateLevelSequencePlayer _fadesequence))
            (Sequencer|Player|Play _returnvalue :!class /Script/MovieScene.MovieSceneSequencePlayer)
            (Variables|/Game/UI_Elements/UI_Widgets/Menus/Cutscene_Widget.Cutscene_Widget_C|SetFadeInActor (Variables|Default|GetWidget) _outactor)
            (Utilities|FlowControl|Delay (Class|TimeManagementBlueprintLibrary|ToSeconds(QualifiedFrameTime) (Media|MediaPlayer|GetDuration _returnvalue))))
          (:Is%20Not%20Valid
            _))
        (UserInterface|Viewport|AddtoViewport (Variables|Default|GetWidget) 9)
        (Actor|DestroyActor)))))

(fn ConstructionScript)

(fn GetFadein
  (params (FadeType :type E_FadeTypes%20Enum :default "NewEnumerator0"))
  (switch Utilities|FlowControl|Switch|SwitchonE_FadeTypes FadeType
    (:NewEnumerator0
      (return 0))
    (:NewEnumerator1
      (return "/Game/LevelSequences/LS_FadeIn_White.LS_FadeIn_White"))
    (:NewEnumerator2
      (return "/Game/LevelSequences/LS_FadeIn_Black.LS_FadeIn_Black"))))
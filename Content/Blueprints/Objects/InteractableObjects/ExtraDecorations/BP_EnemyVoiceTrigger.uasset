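; A one-shot trigger actor that makes an assigned enemy speak a line of dialogue when the player character overlaps it.
; BeginPlay caches the game instance and player character, and destroys the trigger if no enemy is assigned.
; Tick polls for overlap rather than using overlap events, then passes the dialogue row name to the enemy, starts its dialogue and destroys itself.
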(event EventBeginPlay
  (bind _asstealth_game_instance (Utilities|Casting|CastToStealthGameInstance (Game|GetGameInstance)))
  (Variables|Default|SetAs%20Stealth%20Game%20Instance _asstealth_game_instance)
  (bind _asstealth_character (Utilities|Casting|CastToStealthCharacter (Game|Player|GetPlayerPawn 0)))
  (Variables|Default|SetAs%20Stealth%20Character _asstealth_character)
  (Utilities|IsValid (Variables|Default|GetEnemyToSaySomething)
    (:Is%20Not%20Valid
      (Actor|DestroyActor))))

(event Collision|EventActorBeginOverlap
  (params (OtherActor :type Actor%20Object%20Reference)))

(event EventTick
  (params (DeltaSeconds :type Float%20%28single-precision%29))
  (bind _enemytosaysomething (Variables|Default|GetEnemyToSaySomething))
  (if (not (Variables|Default|GetbPlayedDialogue))
    (if (Collision|IsOverlappingActor (Variables|Default|GetAs%20Stealth%20Character) :!class /Script/Engine.Actor)
      (Variables|Default|SetbPlayedDialogue true)
      (Utilities|IsValid _enemytosaysomething
        (:Is%20Valid
          (Variables|/Script/Proj_NinjaGame.Enemy|SetStartDialogueRowName _enemytosaysomething (Variables|Default|GetStartDialogueRowName))
          (Class|Enemy|StartDialogue _enemytosaysomething)
          (Actor|DestroyActor))
        (:Is%20Not%20Valid
          (Actor|DestroyActor))))))

(fn ConstructionScript)
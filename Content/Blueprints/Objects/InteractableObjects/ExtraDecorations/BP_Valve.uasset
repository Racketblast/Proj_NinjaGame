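; BP_Valve is an interactable valve decoration that counts toward a valve-turning achievement.
; On Use it plays its audio, increments ValvesTurned on the first BP_ValveCounter found in the level and prints the total.
; The achievement check compares a constant 0 to 22 instead of the count, so ValveAchievement never unlocks and the valve always disables its collision.
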(event Collision|EventActorBeginOverlap
  (params (OtherActor :type Actor%20Object%20Reference)))

(event EventTick
  (params (DeltaSeconds :type Float%20%28single-precision%29)))

(event EventUse
  (params (Player :type Stealth%20Character%20Object%20Reference))
  (Audio|Components|Audio|Play (Variables|Default|GetAudioComponent) 0.0)
  (bind _outactors (Actor|GetAllActorsOfClass "/Game/Blueprints/Objects/InteractableObjects/ExtraDecorations/BP_ValveCounter.BP_ValveCounter_C"))
  (bind _output_get (Variables|/Game/Blueprints/Objects/InteractableObjects/ExtraDecorations/BP_ValveCounter.BP_ValveCounter_C|SetValvesTurned (Utilities|Array|Get(acopy) _outactors) (+ (Variables|/Game/Blueprints/Objects/InteractableObjects/ExtraDecorations/BP_ValveCounter.BP_ValveCounter_C|GetValvesTurned (Utilities|Array|Get(acopy) _outactors)) 1)))
  (Development|PrintText (Utilities|Text|ToText(Integer) _output_get))
  (if (== 0 22)
    (Class|AchievementSubsystem|UnlockAchievement (Subsystems|GetAchievementSubsystem) "Valve_Achievement")
    (else
      (Collision|SetActorEnableCollision false))))

(fn ConstructionScript)
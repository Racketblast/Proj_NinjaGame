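; BP_Note is an interactable note decoration, an open book with a point light that bobs and opens a UI widget when used.
; From BeginPlay, timeline playback alternates forward and reverse in an endless loop, driving the relative location of the mesh and light.
; The Use event shows the mouse cursor, sets UI-only input, then creates the configured widget and adds it to the viewport.
; The input-mode focus references the widget variable before that widget is created.
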(event EventBeginPlay
  (bind _sm_openbook (Variables|Default|GetSM_OpenBook))
  (bind _zaxis (Timeline|zAxisMove Play)
    (:Update
      (Transformation|SetRelativeLocation _sm_openbook _zaxis false false))
    (:Finished
      (bind _zaxis_2 (Timeline|Timeline ReverseFromEnd)
        (:Update
          (Transformation|SetRelativeLocation _sm_openbook _zaxis_2 false false))
        (:Finished
          (Timeline|zAxisMove PlayFromStart))))))

(event Collision|EventActorBeginOverlap
  (params (OtherActor :type Actor%20Object%20Reference)))

(event EventTick
  (params (DeltaSeconds :type Float%20%28single-precision%29)))

(event EventUse
  (params (Player :type Stealth%20Character%20Object%20Reference))
  (bind _returnvalue (Game|GetPlayerController 0))
  (Variables|/Script/Engine.PlayerController|SetbShowMouseCursor _returnvalue true)
  (Input|SetInputModeUIOnly _returnvalue (stale _returnvalue_2) "DoNotLock" false)
  (bind _returnvalue_2 (UserInterface|CreateWidget (Variables|Default|GetClass)))
  (UserInterface|Viewport|AddtoViewport _returnvalue_2 0))

(fn ConstructionScript)